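; BP_TestActor_Test is a test actor Blueprint that does no visible work at runtime as wired.
; BeginPlay sets Width and Heigh to the same value, waits briefly, then calls SetupConeActor, which is empty.
; A disconnected chain, never executed, holds a short delay and a four-part vector expression that would move ConeActorRef using both actors' transforms, Width, Heigh and the cone's Speed.
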(event Custom|SetupConeActor)

(event EventBeginPlay
  (bind _output_get (Variables|Default|SetWidth 2e+01))
  (Variables|Default|SetHeigh _output_get)
  (Utilities|FlowControl|Delay 2.0)
  (CallFunction|SetupConeActor))

(fn ConstructionScript)